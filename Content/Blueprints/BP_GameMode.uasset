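; Game mode for local multiplayer that creates extra players on BeginPlay, gathers PlayerStarts and shows the boss health bar.
; SpawnCharacter replaces a controller's pawn, alternating Assassin and Wizard through a FlipFlop, and adds that player's health and ult bars.
; DespawnCharacter returns the controller to an InitPawn, with both events setting the view to a shared GameCamera.
; A separate SpawnPlayers function, uncalled here, spawns and possesses parent-class pawns.
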(event `self.ReceiveBeginPlay`
  (bind _playercount (`self.PlayerCount`))
  (bind _returnvalue (`|CreateWidget` "/Game/UI/Widgets/W_BossHealthBar.W_BossHealthBar_C"))
  (`UserWidget.AddToViewport` _returnvalue 0)
  (bind _outactors (`GameplayStatics.GetAllActorsOfClass` "/Script/Engine.PlayerStart"))
  (set `self.SpawnPoints` _outactors)
  (while (<= _playercount 3)
    (`/Engine/EditorBlueprintResources/StandardMacros.IncrementInt` _playercount
      (:`  `
        ;[1 1 1] Specify which player is where
        (`GameplayStatics.CreatePlayer` -1)))))

(event `SpawnCharacter`
  (params (`Player Controller` :type "PlayerController Object Reference"))
  (bind _returnvalue (`Controller.K2_GetPawn` `Player Controller`))
  (bind _asbp_player_controller (cast `/Game/Blueprints/BP_PlayerController` `Player Controller` :!pure true))
  (bind _returnvalue_2 (`self.GetTransform`))
  (`/Engine/EditorBlueprintResources/StandardMacros.IsValid` _returnvalue
    (:`Is Valid`
      (`self.K2_DestroyActor` _returnvalue)
      (`/Engine/EditorBlueprintResources/StandardMacros.FlipFlop`
        (:`A`
          (bind _returnvalue_3 (`|SpawnActorFromClass` "/Game/Blueprints/Assassin/BP_Player_Assassin.BP_Player_Assassin_C" _returnvalue_2 "Undefined" "OverrideRootScale" null 0 null))
          (`Controller.Possess` `Player Controller` _returnvalue_3))
        (:`B`
          (bind _returnvalue_4 (`|SpawnActorFromClass` "/Game/Blueprints/Wizard/BP_Player_Wizard.BP_Player_Wizard_C" _returnvalue_2 "Undefined" "OverrideRootScale" null 0 null))
          (`Controller.Possess` `Player Controller` _returnvalue_4)))
      (`PlayerController.SetViewTargetWithBlend` `Player Controller` (`self.GameCamera`) 0.0 "VTBlend_Linear" 0.0 false)
      (`/Engine/EditorBlueprintResources/StandardMacros.IsValid` `Player Controller`
        (:`Is Valid`
          (`UserWidget.AddToViewport` (`/Game/Blueprints/BP_PlayerController.HealthBar` _asbp_player_controller) 0)
          (`UserWidget.AddToViewport` (`/Game/Blueprints/BP_PlayerController.UltBar` _asbp_player_controller) 0))))))

(event `DespawnCharacter`
  (params (PlayerController :type "PlayerController Object Reference"))
  (bind _returnvalue (`Controller.K2_GetPawn` PlayerController))
  (`/Engine/EditorBlueprintResources/StandardMacros.IsValid` _returnvalue
    (:`Is Valid`
      (`self.K2_DestroyActor` _returnvalue)
      (bind _returnvalue_2 (`|SpawnActorFromClass` "/Game/Blueprints/InitPawn.InitPawn_C" (`self.GetTransform`) "Undefined" "OverrideRootScale" null null))
      (`Controller.Possess` PlayerController _returnvalue_2)
      (`PlayerController.SetViewTargetWithBlend` PlayerController (`self.GameCamera`) 0.0 "VTBlend_Linear" 0.0 false))))

(fn `SpawnPlayers`
  (for _index (range 1 4)
    (`GameplayStatics.CreatePlayer` _index))
  (for _index_2 (range 4)
    (bind _returnvalue (`|SpawnActorFromClass` "/Game/Blueprints/BP_Player_Parent.BP_Player_Parent_C" (`KismetMathLibrary.MakeTransform` (0.0 0.0 2000.0)) "Undefined" "OverrideRootScale" null _index_2 null))
    (`Controller.Possess` (`GameplayStatics.GetPlayerController` _index_2) _returnvalue)))

(fn `UserConstructionScript`)