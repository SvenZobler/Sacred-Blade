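; Game mode for the character select screen, handling local player creation and the selection UI.
; On BeginPlay it removes any existing selection widget, creates an additional local player with its own controller, then shows a new W_CharacterSelect owned by player controller 0.
; AddPlayer creates another local player, increments the PlayerAmountGM counter and returns the new controller.
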(event `self.ReceiveBeginPlay`
  (bind _characterselect (`self.CharacterSelect`))
  (`/Engine/EditorBlueprintResources/StandardMacros.IsValid` _characterselect
    (:`Is Valid`
      (`Widget.RemoveFromParent` _characterselect))
    (:`Is Not Valid`
      _))
  (`GameplayStatics.CreatePlayer` -1)
  (bind _returnvalue (`|CreateWidget` "/Game/UI/Widgets/W_CharacterSelect.W_CharacterSelect_C" (`GameplayStatics.GetPlayerController` 0)))
  (bind _output_get (set `self.CharacterSelect` _returnvalue))
  (`UserWidget.AddToViewport` _output_get 0))

(fn `AddPlayer`
  (returns (PlayerController :type "PlayerController Object Reference"))
  (bind _returnvalue (`GameplayStatics.CreatePlayer` -1))
  (`/Engine/EditorBlueprintResources/StandardMacros.IncrementInt` (`self.PlayerAmountGM`)
    (:`  `
      (return _returnvalue))))

(fn `UserConstructionScript`)