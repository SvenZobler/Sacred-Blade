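; BP_EnemyProjectile is an enemy projectile that damages the player on overlap.
; When it overlaps a BP_Player_Parent it calls DamageDebug on that player, and it destroys itself on overlap with any actor.
; Unconnected leftover nodes reference homing on the ProjectileMovement component and a player-relative target position, but none of them run.
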(event `self.ReceiveBeginPlay`)

(event `self.ReceiveActorBeginOverlap`
  (params (OtherActor :type "Actor Object Reference"))
  (bind _asbp_player_parent (cast `/Game/Blueprints/BP_Player_Parent` OtherActor)
    (:`then`
      (`/Game/Blueprints/BP_Player_Parent.DamageDebug` _asbp_player_parent)
      (`self.K2_DestroyActor`))
    (:`CastFailed`
      (`self.K2_DestroyActor`))))

(fn `UserConstructionScript`)