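; Player Ranger character with a held-fire bow attack, a Swiftness buff and an Arrow Volley ultimate, tuned from the T_RangerVars data table.
; Shooting spawns BP_Arrow on a looping timer, which restarts when Swiftness toggles its rate alongside walk speed.
; At full charge, Volley uses a delayed DoN loop to spawn growing BP_Volley waves and sphere-trace damage onto BP_Boss, with Swiftness modifying the wave count.
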(event `self.ReceiveBeginPlay`
  ;[1 1 1] Var Set
  (bind _returnvalue (`|GetDataTableRow` "/Game/Blueprints/Ranger/T_RangerVars.T_RangerVars" "BaseStats")
    (:`then`
      (bind (_swiftnessattackspeed _swiftnessmovespeed _swiftnesscooldown _swiftnessduration _arrowvolleydamage _arrowvolleytickrate _arrowvolleyswiftnessmodifier _arrowvolleyultcost _arrowdamage _arrowspeed _arrowrateoffire) (break `/Game/Blueprints/Ranger/S_RangerVars` _returnvalue))
      (set `self.SwiftnessAttackSpeed` _swiftnessattackspeed)
      (set `self.SwiftnessMoveSpeed` _swiftnessmovespeed)
      (set `self.SwiftnessCooldown` _swiftnesscooldown)
      (set `self.ArrowVolleyDamage` _arrowvolleydamage)
      (set `self.ArrowVolleyTickrate` _arrowvolleytickrate)
      (set `self.ArrowVolleySwiftnessModifier` _arrowvolleyswiftnessmodifier)
      (set `self.ArrowVolleyUltCost` _arrowvolleyultcost)
      (set `self.ArrowDamage` _arrowdamage)
      (set `self.ArrowSpeed` _arrowspeed)
      (set `self.ArrowRateofFire` _arrowrateoffire)
      (set `self.SwiftnessDuration` _swiftnessduration))))

(event `InputAction|Shoot`
  (params (Key :type "Key Structure"))
  ;[1 1 1] Basic Attack
  (:`Pressed`
    (set `self.isShooting` true)
    (`self.ShootArrow`)
    (`self.StartTimerFunction` (delegate `self.ShootFunction`)))
  (:`Released`
    (set `self.isShooting` false)
    (`KismetSystemLibrary.K2_ClearAndInvalidateTimerHandle` (`self.ShootTimer`))))

(event `self.ShootFunction`
  ;[1 1 1] Basic Attack
  (`self.ShootArrow`))

(event `InputAction|BasicAbility`
  (params (Key :type "Key Structure"))
  ;[1 1 1] Swiftness
  (:`Pressed`
    (if (`self.SwiftAvailable`)
      (set `self.isSwift` true)
      (set `self.SwiftAvailable` false)
      (if (`self.isShooting`)
        (`KismetSystemLibrary.K2_ClearAndInvalidateTimerHandle` (`self.ShootTimer`))
        (`self.StartTimerFunction` (delegate `self.ShootFunction`)))
      (`KismetSystemLibrary.K2_SetTimerDelegate` (delegate `SwiftnessCDTimer`) (`self.SwiftnessCooldown`))
      (`KismetSystemLibrary.K2_SetTimerDelegate` (delegate `SwiftMovespeed`) (`self.SwiftnessDuration`))
      (set `CharacterMovementComponent.MaxWalkSpeed` (`self.SwiftnessMoveSpeed`) (`self.CharacterMovement`)))))

(event `SwiftMovespeed`
  ;[1 1 1] Swiftness
  (set `self.isSwift` false)
  (set `CharacterMovementComponent.MaxWalkSpeed` (`self.DefaultWalkSpeed`) (`self.CharacterMovement`))
  (if (`self.isShooting`)
    (`KismetSystemLibrary.K2_ClearAndInvalidateTimerHandle` (`self.ShootTimer`))
    (`self.StartTimerFunction` (delegate `self.ShootFunction`))))

(event `SwiftnessCDTimer`
  ;[1 1 1] Swiftness
  (set `self.SwiftAvailable` true))

(event `InputAction|UltimateAbility`
  (params (Key :type "Key Structure"))
  (bind _volleyamount (`self.VolleyAmount`))
  (bind _volleyamount_2 (`self.VolleyAmount`))
  (bind _returnvalue (+ (`self.VolleyCastLoc`) (* (`self.StartVector`) (`self.RadiusIncreaser`))))
  (bind _returnvalue_2 (select `bool` (`self.isSwift`) :`false` _volleyamount :`true` (+ _volleyamount (`self.ArrowVolleySwiftnessModifier`))))
  ;[1 1 1] Volley
  (:`Pressed`
    (if (== (`self.CurrentUltCharge`) (`self.UltChargeRequired`))
      (set `self.VolleyCastLoc` (`SceneComponent.K2_GetComponentLocation` (`self.VolleyStartPoint`)))
      (bind _counter (`/Engine/EditorBlueprintResources/StandardMacros.Do N` _returnvalue_2 :!label _label)
        (:`Exit`
          (`|SpawnActorFromClass` "/Game/Blueprints/Ranger/BP_Volley.BP_Volley_C" (`KismetMathLibrary.MakeTransform` _returnvalue (struct) (* (1.0 1.0 1.0) (`self.RadiusIncreaser`))) "Undefined" "OverrideRootScale" null _returnvalue_2 null)
          (bind _outhit (`KismetSystemLibrary.SphereTraceSingleForObjects` _returnvalue (+ (`self.VolleyCastLoc`) (* (`self.EndVector`) (`self.RadiusIncreaser`))) (* (`self.VolleyRadius`) (`self.RadiusIncreaser`)) (`|MakeArray` "ObjectTypeQuery2" :!type "EObjectTypeQuery Enum")))
          (bind _asbp_boss (cast `/Game/Blueprints/BP_Boss` (`.HitActor` (`GameplayStatics.BreakHitResult` _outhit)))
            (:`then`
              (`/Game/Blueprints/BP_Boss.TakeDamage` _asbp_boss (`self.ArrowVolleyDamage`)))
            (:`CastFailed`
              _))
          (if (== _counter (select `bool` (`self.isSwift`) :`false` _volleyamount_2 :`true` (+ _volleyamount_2 (`self.ArrowVolleySwiftnessModifier`))))
            (set `self.CurrentUltCharge` 0.0)
            (set `self.RadiusIncreaser` 1.0)
            (set `self.VolleyCastLoc` (0.0 0.0 0.0))
            (goto _label :!via `Reset`)
            (else
              (set `self.RadiusIncreaser` (+ (`self.RadiusIncreaser`) 0.5))
              (`KismetSystemLibrary.Delay` 0.15)
              (goto _label))))))))

(fn `ShootArrow`
  (bind (_returnvalue_location _returnvalue_rotation) (`KismetMathLibrary.BreakTransform` (`SceneComponent.K2_GetComponentToWorld` (`self.ProjSpawnLoc`))))
  (`|SpawnActorFromClass` "/Game/Blueprints/Ranger/BP_Arrow.BP_Arrow_C" (`KismetMathLibrary.MakeTransform` _returnvalue_location _returnvalue_rotation) "Undefined" "OverrideRootScale" null (`self.ArrowDamage`) (`self.ArrowSpeed`) self))

(fn `StartTimerFunction`
  (params (Delegate :type Delegate))
  (bind _returnvalue (`KismetSystemLibrary.K2_SetTimerDelegate` Delegate (select `bool` (`self.isSwift`) :`false` (`self.ArrowRateofFire`) :`true` (`self.SwiftnessAttackSpeed`)) true))
  (set `self.ShootTimer` _returnvalue))

(fn `UserConstructionScript`
  (`parent.UserConstructionScript`))