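; BP_DamageZone is a hazard actor that drains the player's health while they stand inside it.
; Begin overlap casts to BP_Player_Assassin, stores the reference and sets an overlap flag, which any actor's end overlap clears.
; While the flag is set, Tick subtracts a fixed amount from the player's Health each frame, unscaled by delta time, and prints the value.
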(event `self.ReceiveActorBeginOverlap`
  (params (OtherActor :type "Actor Object Reference"))
  (bind _asbp_player_assassin (cast `/Game/Blueprints/Assassin/BP_Player_Assassin` OtherActor))
  (set `self.REFPlayer` _asbp_player_assassin)
  (set `self.IsOverlapping` true))

(event `self.ReceiveActorEndOverlap`
  (params (OtherActor :type "Actor Object Reference"))
  (set `self.IsOverlapping` false))

(event `self.ReceiveTick`
  (params (DeltaSeconds :type "Float (single-precision)"))
  (bind _refplayer (`self.REFPlayer`))
  (if (`self.IsOverlapping`)
    (bind _output_get (set `/Game/Blueprints/BP_Player_Parent.Health` (- (`/Game/Blueprints/BP_Player_Parent.Health` _refplayer) 0.5) _refplayer))
    (`KismetSystemLibrary.PrintString` (`KismetStringLibrary.Conv_DoubleToString` _output_get))))

(fn `UserConstructionScript`)