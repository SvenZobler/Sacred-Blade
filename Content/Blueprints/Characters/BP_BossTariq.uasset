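; Boss Tariq enemy that starts a spinning chase one second after BeginPlay, using timelines to home in on the player.
; GetRandomPlayer actually returns the nearest player.
; Bear traps attach and deal timed repeat damage with a material flash, while a temporary, crosshair-marked multiplier scales damage taken; zero health triggers GameMode Victory.
; Charge and icicle attacks exist, but their triggers are disconnected.
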(event `Icicle Timer`
  (bind _reficiclevolume (`self.REFIcicleVolume`))
  ;[1 1 1] IcicleSpawns
  (`/Game/Blueprints/BP_IcicleVolume.StartIcicleSpawns` _reficiclevolume)
  (`KismetSystemLibrary.Delay` 5.0)
  (`/Game/Blueprints/BP_IcicleVolume.StopIcicleSpawns` _reficiclevolume))

(event `self.ReceiveBeginPlay`
  (set `self.REFOriginalMat` (`PrimitiveComponent.GetMaterial` (`self.Cube`) 0))
  (`KismetSystemLibrary.Delay` 1.0)
  (bind _outactors (`GameplayStatics.GetAllActorsOfClass` "/Game/Blueprints/Characters/BP_Player_Parent.BP_Player_Parent_C"))
  (for _array_element _outactors
    (`KismetArrayLibrary.Array_Add` (`self.REFPlayers`) _array_element))
  (`self.SpinAttack`))

(event `ChargeAttack`
  (bind _returnvalue (`self.K2_GetActorLocation`))
  ;[1 1 1] ChargeAttack
  (bind _playertarget (`self.GetRandomPlayer`))
  (bind _returnvalue_2 (`self.K2_GetActorLocation` _playertarget))
  (`self.K2_SetActorRotation` (`KismetMathLibrary.FindLookAtRotation` _returnvalue _returnvalue_2))
  (set `self.LastPlayerPos.` _returnvalue_2)
  (`KismetSystemLibrary.Delay` 3.0)
  (bind (_direction _newtrack_3) (`Timeline|ChargeTImeline` :!via `PlayFromStart` :!label _label)
    (:`Update`
      (bind _sweephitresult (`self.K2_SetActorLocation` (`KismetMathLibrary.VLerp` _returnvalue (`self.LastPlayerPos.`) _newtrack_3) true))
      (bind _asbp_player_wizard (cast `/Game/Blueprints/Characters/Wizard/BP_Player_Wizard` (`.HitActor` (`GameplayStatics.BreakHitResult` _sweephitresult)))
        (:`then`
          (`/Game/Blueprints/Characters/BP_Player_Parent.TakeDamage` _asbp_player_wizard 100.0)
          (`self.StopCharge`))
        (:`CastFailed`
          (`KismetSystemLibrary.PrintString` "Hello"))))))

(event `StopCharge`
  ;[1 1 1] ChargeAttack
  (goto _label :!via `Stop`))

(event `GetIcicleLocation`
  (bind _returnvalue (`KismetMathLibrary.RandomPointInBoundingBox` (`self.REFCenterBoxLocation`) (1250.0 1250.0 10.0)))
  (`KismetArrayLibrary.Array_Clear` (`self.ArrayOfLocations`))
  (for _ (range (+ (`self.AmountToSpawn`) 1))
    (bind _outhit (`KismetSystemLibrary.LineTraceSingleForObjects` _returnvalue (- _returnvalue (0.0 0.0 1000.0)) (`|MakeArray` "ObjectTypeQuery7" :!type "EObjectTypeQuery Enum")))
    (bind (_bblockinghit _binitialoverlap _time _distance _location) (`GameplayStatics.BreakHitResult` _outhit))
    (`|SpawnActorFromClass` "/Game/Blueprints/Characters/BP_RedCircle.BP_RedCircle_C" (`KismetMathLibrary.MakeTransform` _location) "Undefined" "OverrideRootScale" null null)
    (`KismetArrayLibrary.Array_Add` (`self.ArrayOfLocations`) _location))
  (`self.SpawnIcicle`))

(event `SpawnIcicle`)

(event `SpinAttack`
  ;[1 1 1] SpinAttack
  (bind _playertarget (`self.GetRandomPlayer`))
  (bind (_direction _spinspeed) (`Timeline|SpinTimeline` :`NewTime` 0.0 :!via `PlayFromStart`)
    (:`Update`
      (`self.K2_AddActorLocalRotation` (`KismetMathLibrary.MakeRotator` 0.0 0.0 _spinspeed))
      (`KismetSystemLibrary.Delay` 1.0)
      (bind (_direction_2 _chasespeed) (`Timeline|FollowTimeline` :!via `PlayFromStart`)
        (:`Update`
          (bind _sweephitresult (`self.K2_SetActorLocation` (`KismetMathLibrary.VLerp` (`self.K2_GetActorLocation`) (`self.K2_GetActorLocation` _playertarget) _chasespeed)))
          (bind _asbp_player_wizard (cast `/Game/Blueprints/Characters/Wizard/BP_Player_Wizard` (`.HitActor` (`GameplayStatics.BreakHitResult` _sweephitresult)))
            (:`then`
              (`/Game/Blueprints/Characters/BP_Player_Parent.TakeDamage` _asbp_player_wizard 100.0))
            (:`CastFailed`
              (`KismetSystemLibrary.PrintString` "Hello"))))))))

(event `TrapAttached`
  ;[1 1 1] Trap Timers
  (`self.DamageFlash`)
  (`self.TakeDamage` (`self.TrapDamage`)))

(event `TrapTimer`
  ;[1 1 1] Trap Timers
  (`SceneComponent.SetHiddenInGame` (`self.TrapTargetIcon`) true false)
  (`KismetSystemLibrary.K2_ClearAndInvalidateTimerHandle` (`self.TrapAttachTimer`)))

(event `ShowCrosshair`
  ;[1 1 1] CrosshairPulse
  (`SceneComponent.SetHiddenInGame` (`self.TrapTargetIcon`) false false))

(event `TrapMultiplierResetTimer`
  ;[1 1 1] Trap Timers
  (`/Engine/EditorBlueprintResources/StandardMacros.DecrementFloat` (`self.TrapMutliplier`)))

(event `DamageFlash`
  ;[1 1 1] DamageFlash
  (`PrimitiveComponent.SetMaterial` (`self.Cube`) 0 "/Game/Assets/Materials/M_DamageFlash.M_DamageFlash")
  (`KismetSystemLibrary.Delay` 0.05)
  (`PrimitiveComponent.SetMaterial` (`self.Cube`) 0 (`self.REFOriginalMat`)))

(fn `BossDeath`
  (`/Game/Blueprints/Gameplay/Gameplay-GameMode.Victory` (cast `/Game/Blueprints/Gameplay/Gameplay-GameMode` (`GameplayStatics.GetGameMode`) :!pure true))
  (`self.K2_DestroyActor`))

(fn `GetRandomPlayer`
  (returns (PlayerTarget :type "Pawn Object Reference"))
  (`BlueprintMapLibrary.Map_Clear` (`self.PlayerCheck`))
  (`KismetArrayLibrary.Array_Clear` (`self.ArrayToCheck`))
  (for _array_element (`self.REFPlayers`)
    (bind _returnvalue (`self.GetDistanceTo` _array_element))
    (`BlueprintMapLibrary.Map_Add` (`self.PlayerCheck`) _returnvalue _array_element)
    (`KismetArrayLibrary.Array_Add` (`self.ArrayToCheck`) _returnvalue))
  (return (`BlueprintMapLibrary.Map_Find` (`self.PlayerCheck`) (`.MinValue` (`KismetMathLibrary.MinOfFloatArray` (`self.ArrayToCheck`))))))

(fn `TakeDamage`
  (params (DamageAmount :type "Float (double-precision)"))
  (bind _output_get (set `self.Health` (`KismetMathLibrary.FClamp` (- (`self.Health`) (* DamageAmount (`self.TrapMutliplier`))) 0.0 (`self.Health`))))
  (bind _output_get_2 (set `self.NormalizedHealth` (`KismetMathLibrary.NormalizeToRange` _output_get 0.0 500.0)))
  (if (<= _output_get_2 0.0)
    (`/Engine/EditorBlueprintResources/StandardMacros.DoOnce` false
      (:`Completed`
        (`self.BossDeath`)))))

(fn `TrapAttach`
  (params (TrapDamage :type "Float (double-precision)"))
  (bind (_returnvalue_location _returnvalue_rotation) (`KismetMathLibrary.BreakTransform` (`SceneComponent.K2_GetComponentToWorld` (`self.TrapSocket1`))))
  (set `self.TrapDamage` TrapDamage)
  (`self.TrapAttached`)
  (bind _returnvalue (`KismetSystemLibrary.K2_SetTimer` null "TrapAttached" 0.5 true))
  (set `self.TrapAttachTimer` _returnvalue)
  (bind _returnvalue_2 (`|SpawnActorFromClass` "/Game/Blueprints/Characters/Ranger/BP_BearTrapClosed.BP_BearTrapClosed_C" (`KismetMathLibrary.MakeTransform` _returnvalue_location _returnvalue_rotation) "Undefined" "OverrideRootScale" null null))
  (`self.K2_AttachToComponent` _returnvalue_2 (`self.TrapSocket1`) "TrapSocket1" "KeepWorld" "KeepWorld" "KeepWorld" true)
  (`KismetSystemLibrary.K2_SetTimer` null "TrapTimer" 7.0))

(fn `TrapDamageMultiplier`
  (`self.ShowCrosshair`)
  (`/Engine/EditorBlueprintResources/StandardMacros.IncrementFloat` (`self.TrapMutliplier`)
    (:`  `
      (`KismetSystemLibrary.K2_SetTimer` null "TrapMultiplierResetTimer" (`self.TrapMultiplierTimer`)))))

(fn `UserConstructionScript`)