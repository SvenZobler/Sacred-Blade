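; BP_Bolt is a Wizard projectile that damages bosses on overlap.
; Hitting an actor tagged Boss triggers its damage flash, adds ult charge to the instigating player and applies BoltDamage.
; It then logs the boss's actual damage taken against the player index in the game instance and destroys itself.
; Construction defers to the parent script, and the ProjectileEffect event is left empty.
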(event `self.ProjectileEffect`)

(event `self.ReceiveActorBeginOverlap`
  (params (OtherActor :type "Actor Object Reference"))
  (bind _boltdamage (`self.BoltDamage`))
  (if (`self.ActorHasTag` OtherActor "Boss")
    (bind _asbp_boss (cast `/Game/Blueprints/Characters/BP_Boss` OtherActor))
    (`/Game/Blueprints/Characters/BP_Boss.DamageFlash` _asbp_boss)
    (bind _asbp_player_parent (cast `/Game/Blueprints/Characters/BP_Player_Parent` (`self.Instigator`))
      (:`then`
        (`/Game/Blueprints/Characters/BP_Player_Parent.AddUltCharge` _asbp_player_parent _boltdamage))
      (:`CastFailed`
        _))
    (`/Game/Blueprints/Characters/BP_Boss.TakeDamage` _asbp_boss _boltdamage)
    (bind _asbp_game_info_instance (cast `/Game/Blueprints/AllLevels/BP_GameInfoInstance` (`self.REFGameInstance`))
      (:`then`
        (`/Game/Blueprints/AllLevels/BP_GameInfoInstance.DamageDoneCatalogue` _asbp_game_info_instance (`self.PlayerInt`) (`/Game/Blueprints/Characters/BP_Boss.DamageTakenActual` _asbp_boss)))
      (:`CastFailed`
        _))
    (`self.K2_DestroyActor`)))

(fn `UserConstructionScript`
  (`parent.UserConstructionScript`))