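; Boss actor with health that briefly starts a level icicle attack and destroys itself when health runs out.
; On BeginPlay it finds the icicle volume, starts its spawns, then stops them after a delay.
; TakeDamage updates normalized health, while a separate DamageFlash event briefly swaps the cube's material.
; An older attack that marks random traced points with red circles before spawning icicles remains but is disconnected, alongside empty shot and trap stubs.
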(event `ShotTimer`)

(event `Shoost`)

(event `self.ReceiveBeginPlay`
  (set `self.REFOriginalMat` (`PrimitiveComponent.GetMaterial` (`self.Cube`) 0))
  (`KismetSystemLibrary.Delay` 1.0)
  (bind _outactors (`GameplayStatics.GetAllActorsOfClass` "/Game/Blueprints/BP_IcicleVolume.BP_IcicleVolume_C"))
  (bind _output_get (set `self.REFIcicleVolume` (`|GetArrayItem` _outactors)))
  (`/Game/Blueprints/BP_IcicleVolume.StartIcicleSpawns` _output_get)
  (`KismetSystemLibrary.Delay` 5.0)
  (`/Game/Blueprints/BP_IcicleVolume.StopIcicleSpawns` _output_get))

(event `GetIcicleLocation`
  (bind _returnvalue (`KismetMathLibrary.RandomPointInBoundingBox` (`self.REFCenterBoxLocation`) (1250.0 1250.0 10.0)))
  (`KismetArrayLibrary.Array_Clear` (`self.ArrayOfLocations`))
  (for _ (range (+ (`self.AmountToSpawn`) 1))
    (bind _outhit (`KismetSystemLibrary.LineTraceSingleForObjects` _returnvalue (- _returnvalue (0.0 0.0 1000.0)) (`|MakeArray` "ObjectTypeQuery7" :!type "EObjectTypeQuery Enum")))
    (bind (_bblockinghit _binitialoverlap _time _distance _location) (`GameplayStatics.BreakHitResult` _outhit))
    (`|SpawnActorFromClass` "/Game/Blueprints/Characters/BP_RedCircle.BP_RedCircle_C" (`KismetMathLibrary.MakeTransform` _location) "Undefined" "OverrideRootScale" null null)
    (`KismetArrayLibrary.Array_Add` (`self.ArrayOfLocations`) _location))
  (`self.SpawnIcicle`))

(event `SpawnIcicle`
  (`KismetSystemLibrary.Delay` 2.9)
  (bind _outactors (`GameplayStatics.GetAllActorsOfClass` "/Game/Blueprints/Characters/BP_RedCircle.BP_RedCircle_C"))
  (for _array_element _outactors
    (`self.K2_DestroyActor` _array_element))
  (for _array_element_2 (`self.ArrayOfLocations`)
    (`|SpawnActorFromClass` "/Game/Blueprints/BP_Icicle_OLD.BP_Icicle_OLD_C" (`KismetMathLibrary.MakeTransform` _array_element_2) "Undefined" "OverrideRootScale" null null)))

(event `DamageFlash`
  (`PrimitiveComponent.SetMaterial` (`self.Cube`) 0 "/Game/Assets/Materials/M_DamageFlash.M_DamageFlash")
  (`KismetSystemLibrary.Delay` 0.05)
  (`PrimitiveComponent.SetMaterial` (`self.Cube`) 0 (`self.REFOriginalMat`)))

(fn `BossDeath`
  (`self.K2_DestroyActor`))

(fn `TakeDamage`
  (params (DamageAmount :type "Float (double-precision)"))
  (bind _output_get (set `self.Health` (- (`self.Health`) DamageAmount)))
  (set `self.NormalizedHealth` (`KismetMathLibrary.NormalizeToRange` _output_get 0.0 500.0))
  (if (<= _output_get 0.0)
    (`self.BossDeath`)))

(fn `TrapAttach`)

(fn `UserConstructionScript`)