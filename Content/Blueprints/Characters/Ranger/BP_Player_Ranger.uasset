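; Ranger player character that fires arrows, uses a Swiftness ability and places a bear trap as its ultimate.
; BeginPlay loads ability and arrow stats from the T_RangerVars data table.
; Looping timers drive held-fire shooting and restart when Swiftness starts or ends to change fire rate, while Swiftness also changes walk speed.
; The ultimate spawns BP_BearTrap at full charge; an older arrow volley graph remains disconnected.
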(event `self.ReceiveBeginPlay`
  ;[1 1 1] Var Set
  (`self.SpawnFunction`)
  (bind _returnvalue (`|GetDataTableRow` "/Game/Blueprints/Characters/Ranger/T_RangerVars.T_RangerVars" "BaseStats")
    (:`then`
      (bind (_swiftnessattackspeed _swiftnessmovespeed _swiftnesscooldown _swiftnessduration _arrowvolleydamage _arrowvolleytickrate _arrowvolleyswiftnessmodifier _arrowvolleyultcost _arrowdamage _arrowspeed _arrowrateoffire) (break `/Game/Blueprints/Characters/Ranger/S_RangerVars` _returnvalue))
      (set `self.SwiftnessAttackSpeed` _swiftnessattackspeed)
      (set `self.SwiftnessMoveSpeed` _swiftnessmovespeed)
      (set `self.SwiftnessCooldown` _swiftnesscooldown)
      (set `self.ArrowVolleyDamage` _arrowvolleydamage)
      (set `self.ArrowVolleyTickrate` _arrowvolleytickrate)
      (set `self.ArrowVolleySwiftnessModifier` _arrowvolleyswiftnessmodifier)
      (set `self.ArrowVolleyUltCost` _arrowvolleyultcost)
      (set `self.ArrowDamage` _arrowdamage)
      (set `self.ArrowSpeed` _arrowspeed)
      (set `self.ArrowRateofFire` _arrowrateoffire)
      (set `self.SwiftnessDuration` _swiftnessduration))))

(event `RateofFireClock`
  ;[1 1 1] ArrowTimer
  (`KismetSystemLibrary.K2_SetTimerDelegate` (delegate `RateofFireBoolSetter`) (select `bool` (`self.isSwift`) :`false` (`self.DefaultRateofFire`) :`true` (`self.SwiftnessAttackSpeed`)) true))

(event `RateofFireBoolSetter`
  ;[1 1 1] ArrowTimer
  (set `self.CanFire` true))

(event `InputAction|Shoot`
  (params (Key :type "Key Structure"))
  ;[1 1 1] Arrow
  (:`Pressed`
    (if (`self.CanFire`)
      (set `self.CanFire` false)
      (`self.RateofFireClock`)
      (set `self.isShooting` true)
      (`self.ShootArrow`))
    (`self.StartTimerFunction` (delegate `self.ShootFunction`)))
  (:`Released`
    (set `self.isShooting` false)
    (`KismetSystemLibrary.K2_ClearAndInvalidateTimerHandle` (`self.ShootTimer`))))

(event `self.ShootFunction`
  ;[1 1 1] Arrow
  (`self.ShootArrow`))

(event `InputAction|BasicAbility`
  (params (Key :type "Key Structure"))
  ;[1 1 1] Swiftness
  (:`Pressed`
    (if (`self.SwiftAvailable`)
      (set `self.isSwift` true)
      (set `self.SwiftAvailable` false)
      (if (`self.isShooting`)
        (`KismetSystemLibrary.K2_ClearAndInvalidateTimerHandle` (`self.ShootTimer`))
        (`self.StartTimerFunction` (delegate `self.ShootFunction`)))
      (`KismetSystemLibrary.K2_SetTimerDelegate` (delegate `SwiftnessCDTimer`) (`self.SwiftnessCooldown`))
      (`KismetSystemLibrary.K2_SetTimerDelegate` (delegate `SwiftMovespeed`) (`self.SwiftnessDuration`))
      (set `CharacterMovementComponent.MaxWalkSpeed` (`self.SwiftnessMoveSpeed`) (`self.CharacterMovement`)))))

(event `SwiftMovespeed`
  ;[1 1 1] Swiftness
  (set `self.isSwift` false)
  (set `CharacterMovementComponent.MaxWalkSpeed` (`self.DefaultWalkSpeed`) (`self.CharacterMovement`))
  (if (`self.isShooting`)
    (`KismetSystemLibrary.K2_ClearAndInvalidateTimerHandle` (`self.ShootTimer`))
    (`self.StartTimerFunction` (delegate `self.ShootFunction`))))

(event `SwiftnessCDTimer`
  ;[1 1 1] Swiftness
  (set `self.SwiftAvailable` true))

(event `InputAction|UltimateAbility`
  (params (Key :type "Key Structure"))
  (bind (_returnvalue_location _returnvalue_rotation) (`KismetMathLibrary.BreakTransform` (`SceneComponent.K2_GetComponentToWorld` (`self.ProjSpawnLoc`))))
  (:`Pressed`
    (if (== (`self.CurrentUltCharge`) (`self.UltChargeRequired`))
      (`|SpawnActorFromClass` "/Game/Blueprints/Characters/Ranger/BP_BearTrap.BP_BearTrap_C" (`KismetMathLibrary.MakeTransform` _returnvalue_location _returnvalue_rotation (2.0 2.0 2.0)) "Undefined" "OverrideRootScale" null null)
      (set `self.CurrentUltCharge` 0.0))))

(fn `ShootArrow`
  (bind (_returnvalue_location _returnvalue_rotation) (`KismetMathLibrary.BreakTransform` (`SceneComponent.K2_GetComponentToWorld` (`self.ProjSpawnLoc`))))
  (`|SpawnActorFromClass` "/Game/Blueprints/Characters/Ranger/BP_Arrow.BP_Arrow_C" (`KismetMathLibrary.MakeTransform` _returnvalue_location _returnvalue_rotation) "Undefined" "OverrideRootScale" null (`self.ArrowDamage`) (`self.ArrowSpeed`) self))

(fn `StartTimerFunction`
  (params (Delegate :type Delegate))
  (bind _returnvalue (`KismetSystemLibrary.K2_SetTimerDelegate` Delegate (select `bool` (`self.isSwift`) :`false` (`self.ArrowRateofFire`) :`true` (`self.SwiftnessAttackSpeed`)) true))
  (set `self.ShootTimer` _returnvalue))

(fn `UserConstructionScript`
  (`parent.UserConstructionScript`))