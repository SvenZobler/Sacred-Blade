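; BP_Arrow is the Ranger's arrow projectile, which damages bosses on contact.
; On BeginPlay it feeds its ArrowSpeed into the ProjectileMovement component's initial speed.
; On overlapping an actor tagged Boss, it triggers that boss's damage flash, applies ArrowDamage, grants the same amount as ultimate charge to the instigating player, then destroys itself.
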(event `self.ReceiveBeginPlay`
  (set `ProjectileMovementComponent.InitialSpeed` (`self.ArrowSpeed`) (`self.ProjectileMovement`)))

(event `self.ProjectileEffect`)

(event `self.ReceiveActorBeginOverlap`
  (params (OtherActor :type "Actor Object Reference"))
  (bind _arrowdamage (`self.ArrowDamage`))
  (if (`self.ActorHasTag` OtherActor "Boss")
    (bind _asbp_boss (cast `/Game/Blueprints/Characters/BP_Boss` OtherActor))
    (`/Game/Blueprints/Characters/BP_Boss.DamageFlash` _asbp_boss)
    (bind _asbp_player_parent (cast `/Game/Blueprints/Characters/BP_Player_Parent` (`self.Instigator`))
      (:`then`
        (`/Game/Blueprints/Characters/BP_Player_Parent.AddUltCharge` _asbp_player_parent _arrowdamage))
      (:`CastFailed`
        _))
    (`/Game/Blueprints/Characters/BP_Boss.TakeDamage` _asbp_boss _arrowdamage)
    (`self.K2_DestroyActor`)))

(fn `UserConstructionScript`
  (`parent.UserConstructionScript`))