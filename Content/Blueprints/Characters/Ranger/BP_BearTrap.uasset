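; Ranger bear trap projectile that arms when it lands and catches the dragon boss.
; While in transit it yaws at a random per-frame rate chosen at BeginPlay.
; When projectile movement stops, the TrapArm timeline drives a dynamic material's Control parameter to show arming.
; Overlapping the boss calls its trap damage multiplier and attach functions, passing damage and player index, then destroys the trap, with no check that it has landed.
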(event `self.ReceiveBeginPlay`
  (set `self.RandomRotation` (`KismetMathLibrary.RandomFloatInRange` -1.0 1.0))
  (bind _returnvalue (`PrimitiveComponent.CreateDynamicMaterialInstance` (`self.BearTrap`) 1 "/Game/Assets/Meshes/M_TrapArm.M_TrapArm" "None"))
  (set `self.REFMiddleMaterial` _returnvalue))

(event `self.ReceiveTick`
  (params (DeltaSeconds :type "Float (single-precision)"))
  (if (`self.inTransit`)
    (`self.K2_AddActorLocalRotation` (`KismetMathLibrary.MakeRotator` 0.0 0.0 (`self.RandomRotation`)))))

(event `self.ProjectileMovement.OnProjectileStop`
  (params (ImpactResult :type "HitResult Structure (by ref)"))
  (set `self.inTransit` false)
  (bind (_direction _newtrack_0) (`Timeline|TrapArm` :!via `PlayFromStart`)
    (:`Update`
      (`MaterialInstanceDynamic.SetScalarParameterValue` (`self.REFMiddleMaterial`) "Control" _newtrack_0))))

(event `self.ReceiveActorBeginOverlap`
  (params (OtherActor :type "Actor Object Reference"))
  (if (`self.ActorHasTag` OtherActor "Boss")
    (bind _asbp_dragon_boss (cast `/Game/Blueprints/Characters/BP_DragonBoss` OtherActor))
    (`/Game/Blueprints/Characters/BP_DragonBoss.TrapDamageMultiplier` _asbp_dragon_boss)
    (`/Game/Blueprints/Characters/BP_DragonBoss.TrapAttach` _asbp_dragon_boss (`self.TrapDamage`) (`self.PlayerInt`))
    (`self.K2_DestroyActor`)))

(fn `UserConstructionScript`)