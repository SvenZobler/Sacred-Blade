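; Polar dragon boss that attacks players on looping timers with charges, frost breath and timed icicle-volume spawns.
; GetRandomPlayer actually picks the nearest player to face.
; Charge sweeps along a Timeline lerp toward that player's saved position, while breath ticks damage on cone overlaps confirmed by line trace.
; Attached bear traps deal repeating damage credited to players, a temporary multiplier scales damage taken, and zero health triggers GameMode Victory.
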(event `Icicle Timer`
  (bind _reficiclevolume (`self.REFIcicleVolume`))
  ;[1 1 1] IcicleSpawns
  (`/Game/Blueprints/BP_IcicleVolume.StartIcicleSpawns` _reficiclevolume)
  (`KismetSystemLibrary.Delay` 5.0)
  (`/Game/Blueprints/BP_IcicleVolume.StopIcicleSpawns` _reficiclevolume))

(event `self.ReceiveBeginPlay`
  (bind _asbp_game_info_instance (cast `/Game/Blueprints/AllLevels/BP_GameInfoInstance` (`GameplayStatics.GetGameInstance`)))
  (set `self.REFGameInstance` _asbp_game_info_instance)
  (set `self.REFOriginalMat` (`PrimitiveComponent.GetMaterial` (`self.Mesh`) 0))
  (`KismetSystemLibrary.K2_SetTimerDelegate` (delegate `BossCharge`) 10.0 true)
  (bind _outactors (`GameplayStatics.GetAllActorsOfClass` "/Game/Blueprints/BP_IcicleVolume.BP_IcicleVolume_C"))
  (bind _output_get (set `self.REFIcicleVolume` (`|GetArrayItem` _outactors)))
  (`KismetSystemLibrary.Delay` 0.5)
  (bind _outactors_2 (`GameplayStatics.GetAllActorsOfClass` "/Game/Blueprints/Characters/BP_Player_Parent.BP_Player_Parent_C"))
  (for _array_element _outactors_2
    (`KismetArrayLibrary.Array_Add` (`self.REFPlayers`) _array_element))
  ;[1 1 1] IcicleSpawns
  (`KismetSystemLibrary.K2_SetTimerDelegate` (delegate `Icicle Timer`) 10.0 true)
  (`/Game/Blueprints/BP_IcicleVolume.StartIcicleSpawns` _output_get)
  (`KismetSystemLibrary.K2_SetTimerDelegate` (delegate `TimerBreath`) 14.0 true)
  (`self.FrostBreath`))

(event `TimerBreath`
  (`self.FrostBreath`))

(event `DamageFlash`
  ;[1 1 1] DamageFlash
  (`PrimitiveComponent.SetMaterial` (`self.Mesh`) 0 "/Game/Assets/Meshes/Beserker_Red.Beserker_Red")
  (`KismetSystemLibrary.Delay` 0.05)
  (`PrimitiveComponent.SetMaterial` (`self.Mesh`) 0 (`self.REFOriginalMat`)))

(event `TrapAttached`
  (params (PlayerInt :type Integer))
  (bind _returnvalue (* (`self.TrapMutliplier`) (`self.TrapDamage`)))
  ;[1 1 1] Trap Timers
  (`/Game/Blueprints/AllLevels/BP_GameInfoInstance.DamageDoneCatalogue` (`self.REFGameInstance`) PlayerInt _returnvalue)
  (`self.TakeDamage` _returnvalue))

(event `TrapTimer`
  ;[1 1 1] Trap Timers
  (`SceneComponent.SetHiddenInGame` (`self.TrapTargetIcon1`) true false)
  (`KismetSystemLibrary.K2_ClearAndInvalidateTimerHandle` (`self.TrapAttachTimer`)))

(event `ShowCrosshair`
  ;[1 1 1] CrosshairPulse
  (`SceneComponent.SetHiddenInGame` (`self.TrapTargetIcon1`) false false))

(event `TrapMultiplierResetTimer`
  ;[1 1 1] Trap Timers
  (`/Engine/EditorBlueprintResources/StandardMacros.DecrementFloat` (`self.TrapMutliplier`)))

(event `BossCharge`
  (bind _returnvalue (`self.K2_GetActorLocation`))
  (bind _player (`self.GetRandomPlayer`))
  (bind _returnvalue_2 (`self.K2_GetActorLocation` _player))
  (`self.K2_SetActorRotation` (`KismetMathLibrary.FindLookAtRotation` _returnvalue _returnvalue_2))
  (set `self.LastPlayerPos.` _returnvalue_2)
  (`KismetSystemLibrary.Delay` 3.0)
  (bind _asab_polar_dragon (cast `/Game/Assets/Boss/AB_PolarDragon` (`SkeletalMeshComponent.GetAnimInstance` (`self.Mesh`))))
  (set `/Game/Assets/Boss/AB_PolarDragon.isCharging` true _asab_polar_dragon)
  (bind (_direction _newtrack_3) (`Timeline|Timeline_0` :!via `PlayFromStart` :!label _label)
    (:`Update`
      (bind _sweephitresult (`self.K2_SetActorLocation` (`KismetMathLibrary.VLerp` _returnvalue (`self.LastPlayerPos.`) _newtrack_3) true))
      (bind _asbp_player_parent (cast `/Game/Blueprints/Characters/BP_Player_Parent` (`.HitActor` (`GameplayStatics.BreakHitResult` _sweephitresult))))
      (`/Game/Blueprints/Characters/BP_Player_Parent.TakeDamage` _asbp_player_parent 20.0)
      (`self.Stop`))
    (:`Finished`
      _))
  (bind _asab_polar_dragon_2 (cast `/Game/Assets/Boss/AB_PolarDragon` (`SkeletalMeshComponent.GetAnimInstance` (`self.Mesh`))))
  (set `/Game/Assets/Boss/AB_PolarDragon.isCharging` true _asab_polar_dragon_2))

(event `Stop`
  (goto _label :!via `Stop`))

(event `self.FrostBreathCone.OnComponentBeginOverlap`
  (params (OverlappedComponent :type "PrimitiveComponent Object Reference") (OtherActor :type "Actor Object Reference") (OtherComp :type "PrimitiveComponent Object Reference") (OtherBodyIndex :type Integer) (bFromSweep :type Boolean) (SweepResult :type "HitResult Structure (by ref)")))

(event `self.FrostBreathCone.OnComponentEndOverlap`
  (params (OverlappedComponent :type "PrimitiveComponent Object Reference") (OtherActor :type "Actor Object Reference") (OtherComp :type "PrimitiveComponent Object Reference") (OtherBodyIndex :type Integer))
  (cast `/Game/Blueprints/Characters/BP_Player_Parent` OtherActor))

(event `FrostBreath`
  (bind _frostbreathcone (`self.FrostBreathCone`))
  ;[1 1 1] Frost Breath
  (bind _asab_polar_dragon (cast `/Game/Assets/Boss/AB_PolarDragon` (`SkeletalMeshComponent.GetAnimInstance` (`self.Mesh`))))
  (set `/Game/Assets/Boss/AB_PolarDragon.isBreathingFrost` true _asab_polar_dragon)
  (bind _player (`self.GetRandomPlayer`))
  (`/Engine/EditorBlueprintResources/StandardMacros.IsValid` _player
    (:`Is Valid`
      (`self.K2_SetActorRotation` (`KismetMathLibrary.FindLookAtRotation` (`SceneComponent.K2_GetComponentLocation` (`self.LookAt`)) (`self.K2_GetActorLocation` _player)))
      (`SceneComponent.SetHiddenInGame` _frostbreathcone false false)
      (`PrimitiveComponent.SetCollisionEnabled` _frostbreathcone "QueryAndPhysics")
      (bind _returnvalue (`KismetSystemLibrary.K2_SetTimerDelegate` (delegate `BreathTick`) (`self.BreathTickInterval`) true))
      (bind _returnvalue_2 (`KismetSystemLibrary.K2_SetTimerDelegate` (delegate `BreathStop`) (`self.FrostBreathDuration`))))))

(event `BreathStop`
  (bind _frostbreathcone (`self.FrostBreathCone`))
  ;[1 1 1] Frost Breath
  (`KismetSystemLibrary.K2_ClearAndInvalidateTimerHandle` (stale `FrostBreath` _returnvalue_2))
  (`KismetSystemLibrary.K2_ClearAndInvalidateTimerHandle` (stale `FrostBreath` _returnvalue))
  (`SceneComponent.SetHiddenInGame` _frostbreathcone true false)
  (`PrimitiveComponent.SetCollisionEnabled` _frostbreathcone "NoCollision")
  (bind _asab_polar_dragon (cast `/Game/Assets/Boss/AB_PolarDragon` (`SkeletalMeshComponent.GetAnimInstance` (`self.Mesh`))))
  (set `/Game/Assets/Boss/AB_PolarDragon.isBreathingFrost` false _asab_polar_dragon))

(event `BreathTick`
  ;[1 1 1] Frost Breath
  (for _array_element (`PrimitiveComponent.GetOverlappingActors` (`self.FrostBreathCone`) "/Game/Blueprints/Characters/BP_Player_Parent.BP_Player_Parent_C")
    (bind _outhit (`KismetSystemLibrary.LineTraceSingleForObjects` (`self.K2_GetActorLocation`) (`self.K2_GetActorLocation` _array_element) (`|MakeArray` "ObjectTypeQuery1" "ObjectTypeQuery3" :!type "EObjectTypeQuery Enum")))
    (bind (_bblockinghit _binitialoverlap _time _distance _location _impactpoint _normal _impactnormal _physmat _hitactor) (`GameplayStatics.BreakHitResult` _outhit))
    (if (`self.ActorHasTag` _hitactor "Player")
      (bind _asbp_player_parent (cast `/Game/Blueprints/Characters/BP_Player_Parent` _hitactor))
      (`/Engine/EditorBlueprintResources/StandardMacros.IsValid` _asbp_player_parent
        (:`Is Valid`
          (`/Game/Blueprints/Characters/BP_Player_Parent.TakeDamage` _asbp_player_parent (`self.FrostBreathTickDamage`)))))))

(fn `BossDeath`
  (`/Game/Blueprints/Gameplay/Gameplay-GameMode.Victory` (cast `/Game/Blueprints/Gameplay/Gameplay-GameMode` (`GameplayStatics.GetGameMode`) :!pure true))
  (`self.K2_DestroyActor`))

(fn `GetRandomPlayer`
  (returns (Player :type "Pawn Object Reference"))
  (`BlueprintMapLibrary.Map_Clear` (`self.PlayerCheck`))
  (`KismetArrayLibrary.Array_Clear` (`self.ArrayToCheck`))
  (for _array_element (`self.REFPlayers`)
    (bind _returnvalue (`self.GetDistanceTo` _array_element))
    (`BlueprintMapLibrary.Map_Add` (`self.PlayerCheck`) _returnvalue _array_element)
    (`KismetArrayLibrary.Array_Add` (`self.ArrayToCheck`) _returnvalue))
  (return (`BlueprintMapLibrary.Map_Find` (`self.PlayerCheck`) (`.MinValue` (`KismetMathLibrary.MinOfFloatArray` (`self.ArrayToCheck`))))))

(fn `TakeDamage`
  (params (Damage :type "Float (double-precision)"))
  (bind _returnvalue (* Damage (`self.TrapMutliplier`)))
  (set `self.DamageTakenActual` _returnvalue)
  (bind _output_get (set `self.Health` (`KismetMathLibrary.FClamp` (- (`self.Health`) _returnvalue) 0.0 (`self.Health`))))
  (bind _output_get_2 (set `self.NormalizedHealth` (`KismetMathLibrary.NormalizeToRange` _output_get 0.0 (`self.TotalHealth`))))
  (if (<= _output_get_2 0.0)
    (`/Engine/EditorBlueprintResources/StandardMacros.DoOnce` false
      (:`Completed`
        (`self.BossDeath`)))))

(fn `TrapAttach`
  (params (TrapDamage :type "Float (double-precision)") (PlayerInt :type Integer))
  (bind (_returnvalue_location _returnvalue_rotation) (`KismetMathLibrary.BreakTransform` (`SceneComponent.K2_GetComponentToWorld` (`self.TrapSocket1`))))
  (set `self.TrapDamage` TrapDamage)
  (`self.TrapAttached` PlayerInt)
  (bind _returnvalue (`KismetSystemLibrary.K2_SetTimer` null "TrapAttached" 0.5 true))
  (set `self.TrapAttachTimer` _returnvalue)
  (bind _returnvalue_2 (`|SpawnActorFromClass` "/Game/Blueprints/Characters/Ranger/BP_BearTrapClosed.BP_BearTrapClosed_C" (`KismetMathLibrary.MakeTransform` _returnvalue_location _returnvalue_rotation) "Undefined" "OverrideRootScale" null null))
  (`self.K2_AttachToComponent` _returnvalue_2 (`self.TrapSocket1`) "TrapSocket1" "KeepWorld" "KeepWorld" "KeepWorld" true)
  (`KismetSystemLibrary.K2_SetTimer` null "TrapTimer" 7.0))

(fn `TrapDamageMultiplier`
  (`self.ShowCrosshair`)
  (`/Engine/EditorBlueprintResources/StandardMacros.IncrementFloat` (`self.TrapMutliplier`)
    (:`  `
      (`KismetSystemLibrary.K2_SetTimer` null "TrapMultiplierResetTimer" (`self.TrapMultiplierTimer`)))))

(fn `UserConstructionScript`)