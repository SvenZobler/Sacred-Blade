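; BP_Kunai is the Assassin's kunai projectile, which damages bosses and is destroyed on overlapping a Boss- or Wall-tagged actor.
; Boss hits trigger a damage flash, add ult charge to the player instigator, log damage to the game instance, apply damage and spawn blood.
; Damage is logged from the boss's DamageTakenActual before TakeDamage runs.
; Wall hits only spawn sparks before destroying the kunai.
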(event `self.ProjectileEffect`)

(event `self.ReceiveActorBeginOverlap`
  (params (OtherActor :type "Actor Object Reference"))
  (bind _kunaidamage (`self.KunaiDamage`))
  (if (`self.ActorHasTag` OtherActor "Boss")
    (bind _asbp_boss (cast `/Game/Blueprints/Characters/BP_Boss` OtherActor))
    (`/Game/Blueprints/Characters/BP_Boss.DamageFlash` _asbp_boss)
    (bind _asbp_player_parent (cast `/Game/Blueprints/Characters/BP_Player_Parent` (`self.Instigator`))
      (:`then`
        (`/Game/Blueprints/Characters/BP_Player_Parent.AddUltCharge` _asbp_player_parent _kunaidamage)
        (bind _asbp_game_info_instance (cast `/Game/Blueprints/AllLevels/BP_GameInfoInstance` (`self.REFGameInstance`))
          (:`then`
            (`/Game/Blueprints/AllLevels/BP_GameInfoInstance.DamageDoneCatalogue` _asbp_game_info_instance (`self.PlayerInt`) (`/Game/Blueprints/Characters/BP_Boss.DamageTakenActual` _asbp_boss) :!label _label)
            (`/Game/Blueprints/Characters/BP_Boss.TakeDamage` _asbp_boss _kunaidamage)
            (`GameplayStatics.SpawnEmitterAtLocation` "/Game/Assets/Weapon/P_Blood.P_Blood" (`self.K2_GetActorLocation`))
            (`self.K2_DestroyActor` :!label _label_2))
          (:`CastFailed`
            (`KismetSystemLibrary.PrintString` "Fail"))))
      (:`CastFailed`
        (goto _label)))
    (elif (`self.ActorHasTag` OtherActor "Wall")
      (`GameplayStatics.SpawnEmitterAtLocation` "/Game/Assets/Weapon/Spark_P.Spark_P" (`self.K2_GetActorLocation`))
      (goto _label_2))))

(fn `UserConstructionScript`
  (`parent.UserConstructionScript`))