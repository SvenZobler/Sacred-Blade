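; Assassin's spinning shuriken projectile that grows on spawn, shrinks on a fixed timer and destroys itself after its lifespan.
; Overlapping an actor tagged Boss halves its velocity and starts a looping damage timer; leaving doubles the velocity and clears the timer.
; Each tick of that timer flashes the boss, logs damage per player in the game instance and applies shuriken damage.
; SetOnFire swaps in a hot-metal material and multiplies the damage.
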(event `self.ReceiveBeginPlay`
  (`KismetSystemLibrary.K2_SetTimerDelegate` (delegate `ShrinkTimeline`) 4.45)
  (bind (_direction _newtrack_0) (`Timeline|SizeIncrease` :!via `PlayFromStart`)
    (:`Update`
      (`self.SetActorScale3D` _newtrack_0))
    (:`Finished`
      (`KismetSystemLibrary.Delay` (`self.ShurikenLifespan`))
      (`self.K2_DestroyActor`))))

(event `ShrinkTimeline`
  (bind (_direction _newtrack_0) (`Timeline|Shrink` :!via `PlayFromStart`)
    (:`Update`
      (`self.SetActorScale3D` _newtrack_0))))

(event `self.ReceiveTick`
  (params (DeltaSeconds :type "Float (single-precision)"))
  (`self.K2_AddActorLocalRotation` (struct :`Yaw` 5.0)))

(event `self.ReceiveActorBeginOverlap`
  (params (OtherActor :type "Actor Object Reference"))
  (bind _projectilemovement (`self.ProjectileMovement`))
  ;[1 1 1] Start Damage Timer Invalidate on End Overlap
  (`/Engine/EditorBlueprintResources/StandardMacros.IsValid` OtherActor
    (:`Is Valid`
      (if (`self.ActorHasTag` OtherActor "Boss")
        (bind _asbp_boss (cast `/Game/Blueprints/Characters/BP_Boss` OtherActor))
        (set `self.REFBoss` _asbp_boss)
        (set `MovementComponent.Velocity` (* (`MovementComponent.Velocity` _projectilemovement) 0.5) _projectilemovement)
        (bind _returnvalue (`KismetSystemLibrary.K2_SetTimerDelegate` (delegate `ShurikenDoT`) (`self.ShurikenDoTTimer`) true))))))

(event `self.ReceiveActorEndOverlap`
  (params (OtherActor :type "Actor Object Reference"))
  (bind _projectilemovement (`self.ProjectileMovement`))
  ;[1 1 1] Start Damage Timer Invalidate on End Overlap
  (if (`self.ActorHasTag` OtherActor "Boss")
    (set `MovementComponent.Velocity` (* (`MovementComponent.Velocity` _projectilemovement) 2.0) _projectilemovement)
    (`KismetSystemLibrary.K2_ClearAndInvalidateTimerHandle` (stale `self.ReceiveActorBeginOverlap` _returnvalue))))

(event `ShurikenDoT`
  (bind _refboss (`self.REFBoss`))
  ;[1 1 1] Damage Feedback
  (`/Game/Blueprints/Characters/BP_Boss.DamageFlash` _refboss)
  (`/Game/Blueprints/AllLevels/BP_GameInfoInstance.DamageDoneCatalogue` (cast `/Game/Blueprints/AllLevels/BP_GameInfoInstance` (`self.GameInstance`) :!pure true) (`self.PlayerInt`) (`/Game/Blueprints/Characters/BP_Boss.DamageTakenActual` _refboss))
  (`/Game/Blueprints/Characters/BP_Boss.TakeDamage` _refboss (`self.ShurikenDamage`)))

(fn `SetOnFire`
  (bind _shuriken (`self.Shuriken`))
  ;[1 1 1] Skel/Vert Particle System
  (`PrimitiveComponent.SetMaterial` _shuriken 0 "/Game/Assets/Materials/M_HotMetal.M_HotMetal")
  (`PrimitiveComponent.SetMaterial` _shuriken 1 "/Game/Assets/Materials/M_HotMetal.M_HotMetal")
  (set `self.ShurikenDamage` (* (`self.ShurikenDamage`) (`self.ShurikenFireMultiplier`))))

(fn `UserConstructionScript`)