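; Berserker's thrown boomerang axe, a randomly spinning projectile that flies until it bounces off a Wall-tagged actor, then homes back to the player.
; The return uses a per-tick lerp scaled by distance, boss overlap and a timeline-driven speed multiplier.
; Boss overlap slows it and starts a looping timer that damages BP_DragonBoss, logs damage and builds ult charge.
; Two collision components stop the spin and destroy the axe upon reaching the player.
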(event `self.ProjectileMovement.OnProjectileBounce`
  (params (ImpactResult :type "HitResult Structure (by ref)") (ImpactVelocity :type "Vector Structure (by ref)"))
  (if (`self.ActorHasTag` (`.HitActor` (`GameplayStatics.BreakHitResult` ImpactResult)) "Wall")
    (`ActorComponent.SetActive` (`self.ProjectileMovement`) false false)
    (`GameplayStatics.SpawnEmitterAtLocation` "/Game/Assets/Weapon/Spark_P.Spark_P" (`self.K2_GetActorLocation`))
    (`PrimitiveComponent.SetCollisionEnabled` (`self.StopSpinCollision`) "QueryOnly")
    (`PrimitiveComponent.SetCollisionEnabled` (`self.DestroyActorCollision`) "QueryOnly")
    (set `self.Returning` true)))

(event `self.ReceiveTick`
  (params (DeltaSeconds :type "Float (single-precision)"))
  (bind _refplayer (`self.REFPlayer`))
  (`self.K2_AddActorLocalRotation` (`KismetMathLibrary.MakeRotator` 0.0 0.0 (`self.RandomRotation`)))
  (if (`self.Returning`)
    (`SceneComponent.K2_SetWorldLocation` (`self.Sphere`) (`KismetMathLibrary.VLerp` (`SceneComponent.K2_GetComponentLocation` (`self.Sphere`)) (`self.K2_GetActorLocation` _refplayer) (* (* (* DeltaSeconds (`KismetMathLibrary.MapRangeClamped` (`self.GetDistanceTo` _refplayer) 0.0 5000.0 4.5 0.1)) (`self.OverlapTickMultiplier`)) (`self.LifespanSpeedIncrease`))) false false)))

(event `self.ReceiveActorBeginOverlap`
  (params (OtherActor :type "Actor Object Reference"))
  (bind _projectilemovement (`self.ProjectileMovement`))
  (if (`self.ActorHasTag` OtherActor "Boss")
    (set `self.REFBoss` OtherActor)
    (set `self.OverlapTickMultiplier` (`self.OverlapBeginTickMultiplier`))
    (set `MovementComponent.Velocity` (* (`MovementComponent.Velocity` _projectilemovement) (`self.OverlapVelocityReducer`)) _projectilemovement)
    (bind _returnvalue (`KismetSystemLibrary.K2_SetTimerDelegate` (delegate `OverlapTimer`) 0.1 true))
    (set `self.DamageTimer` _returnvalue)))

(event `self.ReceiveBeginPlay`
  (set `self.RandomRotation` (`KismetMathLibrary.RandomFloatInRange` 6.0 10.0)))

(event `OverlapTimer`
  (bind _asbp_dragon_boss (cast `/Game/Blueprints/Characters/BP_DragonBoss` (`self.REFBoss`)))
  (`/Game/Blueprints/Characters/BP_DragonBoss.DamageFlash` _asbp_dragon_boss)
  (`/Game/Blueprints/Characters/BP_DragonBoss.TakeDamage` _asbp_dragon_boss (`self.AxeDamage`))
  (bind _asbp_game_info_instance (cast `/Game/Blueprints/AllLevels/BP_GameInfoInstance` (`self.REFGameInstance`))
    (:`then`
      (`/Game/Blueprints/AllLevels/BP_GameInfoInstance.DamageDoneCatalogue` _asbp_game_info_instance (`self.PlayerInt`) (`/Game/Blueprints/Characters/BP_DragonBoss.DamageTakenActual` _asbp_dragon_boss)))
    (:`CastFailed`
      _))
  (bind _asbp_player_parent (cast `/Game/Blueprints/Characters/BP_Player_Parent` (`self.REFPlayer`)))
  (`/Game/Blueprints/Characters/BP_Player_Parent.AddUltCharge` _asbp_player_parent (`self.AxeDamage`))
  (`GameplayStatics.SpawnEmitterAtLocation` "/Game/Assets/Weapon/P_Blood.P_Blood" (`SceneComponent.K2_GetComponentLocation` (`self.Scene`))))

(event `self.StopSpinCollision.OnComponentBeginOverlap`
  (params (OverlappedComponent :type "PrimitiveComponent Object Reference") (OtherActor :type "Actor Object Reference") (OtherComp :type "PrimitiveComponent Object Reference") (OtherBodyIndex :type Integer) (bFromSweep :type Boolean) (SweepResult :type "HitResult Structure (by ref)"))
  (if (== OtherActor (`self.REFPlayer`))
    (set `self.RandomRotation` 0.0)))

(event `self.ReceiveActorEndOverlap`
  (params (OtherActor :type "Actor Object Reference"))
  (bind _projectilemovement (`self.ProjectileMovement`))
  (if (`self.ActorHasTag` OtherActor "Boss")
    (`KismetSystemLibrary.K2_ClearAndInvalidateTimerHandle` (`self.DamageTimer`))
    (set `self.OverlapTickMultiplier` (`self.OverlapEndVelocityReset`))
    (set `MovementComponent.Velocity` (* (`MovementComponent.Velocity` _projectilemovement) 3.0) _projectilemovement)))

(event `self.DestroyActorCollision.OnComponentBeginOverlap`
  (params (OverlappedComponent :type "PrimitiveComponent Object Reference") (OtherActor :type "Actor Object Reference") (OtherComp :type "PrimitiveComponent Object Reference") (OtherBodyIndex :type Integer) (bFromSweep :type Boolean) (SweepResult :type "HitResult Structure (by ref)"))
  (if (== OtherActor (`self.REFPlayer`))
    (`self.K2_DestroyActor`)))

(event `SpeedIncreaser`
  (bind (_direction _newtrack_0) (`Timeline|Increaser` :!via `PlayFromStart`)
    (:`Update`
      (set `self.LifespanSpeedIncrease` _newtrack_0))))

(fn `UserConstructionScript`)