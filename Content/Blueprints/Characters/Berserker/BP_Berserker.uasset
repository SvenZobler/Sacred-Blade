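; Playable Berserker character that loads its damage, cooldown and rage tuning from the T_BerserkerVars data table on BeginPlay.
; Shoot throws BP_Axe projectiles on looping timers, and the basic ability spawns a BP_Boomeraxe gated by a cooldown timer.
; At full charge, the ultimate attaches two BP_UltAxes for the rage duration, turning Shoot into alternating sphere-trace melee hits on BP_Boss.
; The debug timer and local chevron widget setup are left unused.
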(event `self.ReceiveBeginPlay`
  (set `self.Character` "Berserker")
  (set `self.PlayerController_0` (`GameplayStatics.GetPlayerController` (`self.PlayerInt`)))
  (`self.SpawnFunction`)
  (bind _returnvalue (`|GetDataTableRow` "/Game/Blueprints/Characters/Berserker/T_BerserkerVars.T_BerserkerVars" "DefaultVars")
    (:`then`
      (bind (_axedamage _axecooldown _boomeraxedamage _boomeraxecooldown _rageattackdamage _rageduration) (break `/Game/Blueprints/Characters/Berserker/S_BerserkerVars` _returnvalue))
      (set `self.AxeDamage` _axedamage)
      (set `self.AxeCooldown` _axecooldown)
      (set `self.BoomeraxeDamage` _boomeraxedamage)
      (set `self.BoomeraxeCooldown` _boomeraxecooldown)
      (set `self.RageAttackDamage` _rageattackdamage)
      (set `self.RageDuration` _rageduration)
      (`self.ChevronSet` (`GameplayStatics.GetPlayerController` (`self.PlayerInt`))))))

(event `Timer`
  (`KismetSystemLibrary.K2_SetTimerDelegate` (delegate `Debug`) 0.2 true))

(event `Debug`
  (`KismetSystemLibrary.PrintString` (`KismetStringLibrary.Conv_VectorToString` (`SceneComponent.GetForwardVector` (`self.Arrow1`)))))

(event `RateofFireClock`
  ;[1 1 1] AxeTimer
  (`KismetSystemLibrary.K2_SetTimerDelegate` (delegate `RateofFireBoolSetter`) 0.49 true))

(event `InputAction|Shoot`
  (params (Key :type "Key Structure"))
  (bind _returnvalue (`SceneComponent.K2_GetComponentLocation` (`self.AxeLoc2`)))
  (bind _returnvalue_2 (`SceneComponent.K2_GetComponentLocation` (`self.AxeLoc1`)))
  ;[1 1 1] Axe
  (:`Pressed`
    (if (`self.isUlting`)
      ;[1 1 1] RageMeleeChange
      (`/Engine/EditorBlueprintResources/StandardMacros.FlipFlop`
        (:`A`
          (bind _outhit (`KismetSystemLibrary.SphereTraceSingleForObjects` :`Start` _returnvalue_2 :`End` (+ _returnvalue_2 (200.0 0.0 0.0)) :`Radius` 250.0 :`ObjectTypes` (`|MakeArray` "ObjectTypeQuery7" :!type "EObjectTypeQuery Enum") :`DrawDebugType` "ForDuration"))
          (bind _asbp_boss (cast `/Game/Blueprints/Characters/BP_Boss` (`.HitActor` (`GameplayStatics.BreakHitResult` _outhit))))
          (`/Game/Blueprints/Characters/BP_Boss.DamageFlash` _asbp_boss)
          (`/Game/Blueprints/Characters/BP_Boss.TakeDamage` _asbp_boss (`self.RageAttackDamage`)))
        (:`B`
          (bind _outhit_2 (`KismetSystemLibrary.SphereTraceSingleForObjects` :`Start` _returnvalue :`End` (+ _returnvalue (200.0 0.0 0.0)) :`Radius` 250.0 :`ObjectTypes` (`|MakeArray` "ObjectTypeQuery7" :!type "EObjectTypeQuery Enum") :`DrawDebugType` "ForDuration"))
          (bind _asbp_boss_2 (cast `/Game/Blueprints/Characters/BP_Boss` (`.HitActor` (`GameplayStatics.BreakHitResult` _outhit_2))))
          (`/Game/Blueprints/Characters/BP_Boss.DamageFlash` _asbp_boss_2)
          (`/Game/Blueprints/Characters/BP_Boss.TakeDamage` _asbp_boss_2 (`self.RageAttackDamage`))))
      (else
        (if (`self.CanFire`)
          (set `self.CanFire` false)
          (`self.RateofFireClock`)
          (`self.BerserkerProj`))
        (bind _returnvalue_3 (`KismetSystemLibrary.K2_SetTimerDelegate` (delegate `self.ShootFunction`) 0.5 true)))))
  (:`Released`
    (`KismetSystemLibrary.K2_ClearAndInvalidateTimerHandle` _returnvalue_3)))

(event `RateofFireBoolSetter`
  ;[1 1 1] AxeTimer
  (set `self.CanFire` true))

(event `self.ShootFunction`
  ;[1 1 1] Axe
  (`self.BerserkerProj`))

(event `InputAction|BasicAbility`
  (params (Key :type "Key Structure"))
  (bind (_returnvalue_location _returnvalue_rotation) (`KismetMathLibrary.BreakTransform` (`SceneComponent.K2_GetComponentToWorld` (`self.ProjSpawnLoc`))))
  ;[1 1 1] Boomeraxe
  (:`Pressed`
    (if (`self.BoomeraxeReady`)
      (`|SpawnActorFromClass` "/Game/Blueprints/Characters/Berserker/BP_Boomeraxe.BP_Boomeraxe_C" (`KismetMathLibrary.MakeTransform` _returnvalue_location _returnvalue_rotation) "Undefined" "OverrideRootScale" null self (`self.BoomeraxeDamage`) self)
      ;[1 1 1] CherryBombCooldown
      (set `self.BoomeraxeReady` false)
      (`KismetSystemLibrary.K2_SetTimerDelegate` (delegate `CherryBombCDTimer`) (`self.BoomeraxeCooldown`)))))

(event `CherryBombCDTimer`
  ;[1 1 1] CherryBombCooldown
  (set `self.BoomeraxeReady` true))

(event `InputAction|UltimateAbility`
  (params (Key :type "Key Structure"))
  (bind _axeloc1 (`self.AxeLoc1`))
  (bind _axeloc2 (`self.AxeLoc2`))
  ;[1 1 1] Wicko Mode
  (:`Pressed`
    (if (== (`self.CurrentUltCharge`) (`self.UltChargeRequired`))
      (set `self.isUlting` true)
      (`KismetSystemLibrary.K2_ClearAndInvalidateTimerHandle` (stale `InputAction|Shoot` _returnvalue_3))
      (bind _returnvalue (`|SpawnActorFromClass` "/Game/Blueprints/Characters/Berserker/BP_UltAxes.BP_UltAxes_C" (`KismetMathLibrary.MakeTransform` (`SceneComponent.K2_GetComponentLocation` _axeloc1)) "Undefined" "OverrideRootScale" null null))
      (`self.K2_AttachToComponent` _returnvalue _axeloc1 "AxeLoc1" "KeepWorld" "KeepWorld" "KeepWorld" true)
      (bind _returnvalue_2 (`|SpawnActorFromClass` "/Game/Blueprints/Characters/Berserker/BP_UltAxes.BP_UltAxes_C" (`KismetMathLibrary.MakeTransform` (`SceneComponent.K2_GetComponentLocation` _axeloc2)) "Undefined" "OverrideRootScale" null null))
      (`self.K2_AttachToComponent` _returnvalue_2 _axeloc2 "None" "KeepWorld" "KeepWorld" "KeepWorld" true)
      (`KismetSystemLibrary.K2_SetTimerDelegate` (delegate `EndUlt`) (`self.RageDuration`))
      (set `self.CurrentUltCharge` 0.0))))

(event `EndUlt`
  ;[1 1 1] Wicko Mode
  (set `self.isUlting` false)
  (`self.K2_DestroyActor` (stale `InputAction|UltimateAbility` _returnvalue_2))
  (`self.K2_DestroyActor` (stale `InputAction|UltimateAbility` _returnvalue)))

(fn `BerserkerProj`
  (bind (_returnvalue_location _returnvalue_rotation) (`KismetMathLibrary.BreakTransform` (`SceneComponent.K2_GetComponentToWorld` (`self.ProjSpawnLoc`))))
  (`|SpawnActorFromClass` "/Game/Blueprints/Characters/Berserker/BP_Axe.BP_Axe_C" (`KismetMathLibrary.MakeTransform` _returnvalue_location _returnvalue_rotation) "Undefined" "OverrideRootScale" null (`self.AxeDamage`) self))

(fn `ChevronSet_0`)

(fn `UserConstructionScript`
  (`parent.UserConstructionScript`))