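; BP_Axe is the Berserker's spinning axe projectile, which damages bosses on overlap.
; It picks a random pitch spin at BeginPlay and applies it every tick, unscaled by delta time.
; Hitting a Boss flashes it, deals damage, adds ult charge to the instigating player and logs damage in the GameInstance.
; Valid boss hits spawn blood and Wall hits spawn sparks, both destroying the axe.
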(event `self.ReceiveBeginPlay`
  (set `self.RandomRotation` (`KismetMathLibrary.RandomFloatInRange` -3.0 -5.0)))

(event `self.ReceiveActorBeginOverlap`
  (params (OtherActor :type "Actor Object Reference"))
  (bind _returnvalue (`self.K2_GetActorLocation`))
  (bind _axedamage (`self.AxeDamage`))
  (if (`self.ActorHasTag` OtherActor "Boss")
    (bind _asbp_boss (cast `/Game/Blueprints/Characters/BP_Boss` OtherActor))
    (`/Game/Blueprints/Characters/BP_Boss.DamageFlash` _asbp_boss)
    (bind _asbp_player_parent (cast `/Game/Blueprints/Characters/BP_Player_Parent` (`self.Instigator`)))
    (`/Engine/EditorBlueprintResources/StandardMacros.IsValid` _asbp_player_parent
      (:`Is Valid`
        (`/Game/Blueprints/Characters/BP_Player_Parent.AddUltCharge` _asbp_player_parent _axedamage)
        (`/Game/Blueprints/Characters/BP_Boss.TakeDamage` _asbp_boss _axedamage)
        (bind _asbp_game_info_instance (cast `/Game/Blueprints/AllLevels/BP_GameInfoInstance` (`self.REFGameInstance`))
          (:`then`
            (`/Game/Blueprints/AllLevels/BP_GameInfoInstance.DamageDoneCatalogue` _asbp_game_info_instance (`self.PlayerInt`) (`/Game/Blueprints/Characters/BP_Boss.DamageTakenActual` _asbp_boss)))
          (:`CastFailed`
            _))
        (`GameplayStatics.SpawnEmitterAtLocation` "/Game/Assets/Weapon/P_Blood.P_Blood" _returnvalue)
        (`self.K2_DestroyActor` :!label _label)))
    (elif (`self.ActorHasTag` OtherActor "Wall")
      (`GameplayStatics.SpawnEmitterAtLocation` "/Game/Assets/Weapon/Spark_P.Spark_P" _returnvalue)
      (goto _label))))

(event `self.ReceiveTick`
  (params (DeltaSeconds :type "Float (single-precision)"))
  (`self.K2_AddActorLocalRotation` (`KismetMathLibrary.MakeRotator` 0.0 (`self.RandomRotation`))))

(fn `UserConstructionScript`)