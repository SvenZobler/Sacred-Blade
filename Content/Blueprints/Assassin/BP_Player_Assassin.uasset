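; Player Blueprint for the Assassin, handling its kunai shot, cherry bomb ability and shuriken ultimate.
; BeginPlay loads stats from the T_AssassinVars data table, and spawned projectiles receive their damage values from them.
; Kunai repeat on a looping timer while Shoot is held, with hardcoded intervals rather than the loaded fire rate.
; Cherry bomb uses a timed cooldown, while the shuriken requires exactly full ult charge and resets it.
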(event `self.ReceiveBeginPlay`
  (bind _returnvalue (`|GetDataTableRow` "/Game/Blueprints/Assassin/T_AssassinVars.T_AssassinVars" "BaseStats")
    (:`then`
      (bind (_projectiledamage _projectilespeed _projectilerateoffire _cherrybombdamage _cherrybombdirectdamage _cherrybombcooldown _shurikendamage _shurikenfiremultiplier _shurikenultcost _shurikenlifespan) (break `/Game/Blueprints/Assassin/S_AssassinVars` _returnvalue))
      (set `self.ProjectileDamage` _projectiledamage)
      (set `self.ProjectileSpeed` _projectilespeed)
      (set `self.ProjectileRateofFire` _projectilerateoffire)
      (set `self.CherryBombDamage` _cherrybombdamage)
      (set `self.CherryBombDirectDamage` _cherrybombdirectdamage)
      (set `self.CherryBombCooldown` _cherrybombcooldown)
      (set `self.ShurikenDamage` _shurikendamage)
      (set `self.ShurikenFireMultiplier` _shurikenfiremultiplier)
      (set `self.ShurikenUltCost` _shurikenultcost)
      (set `self.ShurikenLifespan` _shurikenlifespan))))

(event `RateofFireClock`
  ;[1 1 1] KunaiTimer
  (`KismetSystemLibrary.K2_SetTimerDelegate` (delegate `RateofFireBoolSetter`) 0.49 true))

(event `RateofFireBoolSetter`
  ;[1 1 1] KunaiTimer
  (set `self.CanFire` true))

(event `InputAction|Shoot`
  (params (Key :type "Key Structure"))
  ;[1 1 1] Kunai
  (:`Pressed`
    (if (`self.CanFire`)
      (set `self.CanFire` false)
      (`self.RateofFireClock`)
      (`self.AssassinProj`))
    (bind _returnvalue (`KismetSystemLibrary.K2_SetTimerDelegate` (delegate `self.ShootFunction`) 0.5 true)))
  (:`Released`
    (`KismetSystemLibrary.K2_ClearAndInvalidateTimerHandle` _returnvalue)))

(event `self.ShootFunction`
  ;[1 1 1] Kunai
  (`self.AssassinProj`))

(event `InputAction|BasicAbility`
  (params (Key :type "Key Structure"))
  (bind (_returnvalue_location _returnvalue_rotation) (`KismetMathLibrary.BreakTransform` (`SceneComponent.K2_GetComponentToWorld` (`self.ProjSpawnLoc`))))
  ;[1 1 1] Cherry Bomb
  (:`Pressed`
    (if (`self.CherryBombReady`)
      (`|SpawnActorFromClass` "/Game/Blueprints/Assassin/BP_CherryBomb.BP_CherryBomb_C" (`KismetMathLibrary.MakeTransform` _returnvalue_location _returnvalue_rotation (3.0 3.0 3.0)) "Undefined" "OverrideRootScale" null (`self.CherryBombDamage`) (`self.CherryBombDirectDamage`) self)
      ;[1 1 1] CherryBombCooldown
      (set `self.CherryBombReady` false)
      (`KismetSystemLibrary.K2_SetTimerDelegate` (delegate `CherryBombCDTimer`) (`self.CherryBombCooldown`)))))

(event `CherryBombCDTimer`
  ;[1 1 1] CherryBombCooldown
  (set `self.CherryBombReady` true))

(event `InputAction|UltimateAbility`
  (params (Key :type "Key Structure"))
  (bind (_returnvalue_location _returnvalue_rotation) (`KismetMathLibrary.BreakTransform` (`SceneComponent.K2_GetComponentToWorld` (`self.ProjSpawnLoc`))))
  ;[1 1 1] Shuriken
  (:`Pressed`
    (if (== (`self.CurrentUltCharge`) (`self.UltChargeRequired`))
      (`|SpawnActorFromClass` "/Game/Blueprints/Assassin/BP_Shuriken.BP_Shuriken_C" (`KismetMathLibrary.MakeTransform` _returnvalue_location _returnvalue_rotation (75.0 75.0 75.0)) "Undefined" "OverrideRootScale" null (`self.ShurikenDamage`) (`self.ShurikenFireMultiplier`) (`self.ShurikenLifespan`) self)
      (set `self.CurrentUltCharge` 0.0)
      (set `self.NormalizedUltCharge` 0.0))))

(fn `AssassinProj`
  (bind (_returnvalue_location _returnvalue_rotation) (`KismetMathLibrary.BreakTransform` (`SceneComponent.K2_GetComponentToWorld` (`self.ProjSpawnLoc`))))
  (`|SpawnActorFromClass` "/Game/Blueprints/Assassin/BP_Kunai.BP_Kunai_C" (`KismetMathLibrary.MakeTransform` _returnvalue_location _returnvalue_rotation) "Undefined" "OverrideRootScale" null (`self.ProjectileDamage`) self))

(fn `UserConstructionScript`
  (`parent.UserConstructionScript`))