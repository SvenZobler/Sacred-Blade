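; BP_FirePatch is a short-lived ground hazard that deals damage over time to the boss and destroys itself after five seconds.
; When a Boss-tagged actor overlaps DamageVolume, it caches the boss and the Instigator player, then starts a looping timer.
; Each tick flashes the boss, applies FireballPatchDamage and adds that amount to the player's ult charge.
; The boss ending its overlap clears the timer.
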(event `self.ReceiveBeginPlay`
  (`KismetSystemLibrary.Delay` 5.0)
  (`self.K2_DestroyActor`))

(event `self.DamageVolume.OnComponentBeginOverlap`
  (params (OverlappedComponent :type "PrimitiveComponent Object Reference") (OtherActor :type "Actor Object Reference") (OtherComp :type "PrimitiveComponent Object Reference") (OtherBodyIndex :type Integer) (bFromSweep :type Boolean) (SweepResult :type "HitResult Structure (by ref)"))
  (if (`self.ActorHasTag` OtherActor "Boss")
    (bind _asbp_boss (cast `/Game/Blueprints/BP_Boss` OtherActor))
    (bind _asbp_player_parent (cast `/Game/Blueprints/BP_Player_Parent` (`self.Instigator`)))
    (bind _returnvalue (`KismetSystemLibrary.K2_SetTimerDelegate` (delegate `DealDoTDamage`) 0.5 true))))

(event `DealDoTDamage`
  (bind _fireballpatchdamage (`self.FireballPatchDamage`))
  (`/Game/Blueprints/BP_Boss.DamageFlash` (stale `self.DamageVolume.OnComponentBeginOverlap` _asbp_boss))
  (`/Game/Blueprints/BP_Player_Parent.AddUltCharge` (stale `self.DamageVolume.OnComponentBeginOverlap` _asbp_player_parent) _fireballpatchdamage)
  (`/Game/Blueprints/BP_Boss.TakeDamage` (stale `self.DamageVolume.OnComponentBeginOverlap` _asbp_boss) _fireballpatchdamage))

(event `self.ReceiveActorEndOverlap`
  (params (OtherActor :type "Actor Object Reference"))
  (if (`self.ActorHasTag` OtherActor "Boss")
    (`KismetSystemLibrary.K2_ClearAndInvalidateTimerHandle` (stale `self.DamageVolume.OnComponentBeginOverlap` _returnvalue))))

(fn `UserConstructionScript`)