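; Wizard player character that fires bolts, casts fireballs and launches a shuriken ultimate from a shared projectile spawn point.
; BeginPlay loads bolt, fireball and beam stats from T_WizardVars, though only the fireball values are used here.
; Held shooting repeats on a hardcoded looping timer, with a CanFire gate on the initial shot.
; FireballStartTimer runs the fireball cooldown but is not called here; the ultimate requires full charge and resets it.
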(event `self.ReceiveBeginPlay`
  (bind _returnvalue (`|GetDataTableRow` "/Game/Blueprints/Wizard/T_WizardVars.T_WizardVars" "BaseStats")
    (:`then`
      (bind (_boltdamage _boltspeed _boltrateoffire _fireballdamage _fireballfirepatchdamage _fireballcooldown _beamdamage _beamlength _beamduration) (break `/Game/Blueprints/Wizard/S_WizardVars` _returnvalue))
      (set `self.BoltDamage` _boltdamage)
      (set `self.BoltSpeed` _boltspeed)
      (set `self.BoltRateofFire` _boltrateoffire)
      (set `self.FireballDamage` _fireballdamage)
      (set `self.FireballPatchDamage` _fireballfirepatchdamage)
      (set `self.FireballCooldown` _fireballcooldown)
      (set `self.BeamDamage` _beamdamage)
      (set `self.BeamLength` _beamlength)
      (set `self.BeamDuration` _beamduration))))

(event `RateofFireClock`
  ;[1 1 1] BoltTimer
  (`KismetSystemLibrary.K2_SetTimerDelegate` (delegate `RateofFireBoolSetter`) 0.49 true))

(event `RateofFireBoolSetter`
  ;[1 1 1] BoltTimer
  (set `self.CanFire` true))

(event `InputAction|Shoot`
  (params (Key :type "Key Structure"))
  ;[1 1 1] Bolt
  (:`Pressed`
    (if (`self.CanFire`)
      (set `self.CanFire` false)
      (`self.RateofFireClock`)
      (`self.BoltProj`))
    (bind _returnvalue (`KismetSystemLibrary.K2_SetTimerDelegate` (delegate `self.ShootFunction`) 0.5 true)))
  (:`Released`
    (`KismetSystemLibrary.K2_ClearAndInvalidateTimerHandle` _returnvalue)))

(event `self.ShootFunction`
  ;[1 1 1] Bolt
  (`self.BoltProj`))

(event `FireballStartTimer`
  ;[1 1 1] FireballCD
  (set `self.FireballReady` false)
  (`KismetSystemLibrary.K2_SetTimerDelegate` (delegate `CherryBombCDTimer`) (`self.FireballCooldown`)))

(event `InputAction|BasicAbility`
  (params (Key :type "Key Structure"))
  (bind (_returnvalue_location _returnvalue_rotation) (`KismetMathLibrary.BreakTransform` (`SceneComponent.K2_GetComponentToWorld` (`self.ProjSpawnLoc`))))
  ;[1 1 1] Fireball
  (:`Pressed`
    (if (`self.FireballReady`)
      (`|SpawnActorFromClass` "/Game/Blueprints/Wizard/BP_Fireball.BP_Fireball_C" (`KismetMathLibrary.MakeTransform` _returnvalue_location _returnvalue_rotation (3.0 3.0 3.0)) "Undefined" "OverrideRootScale" null (`self.FireballDamage`) (`self.FireballPatchDamage`) self))))

(event `CherryBombCDTimer`
  ;[1 1 1] FireballCD
  (set `self.FireballReady` true))

(event `InputAction|UltimateAbility`
  (params (Key :type "Key Structure"))
  (bind (_returnvalue_location _returnvalue_rotation) (`KismetMathLibrary.BreakTransform` (`SceneComponent.K2_GetComponentToWorld` (`self.ProjSpawnLoc`))))
  ;[1 1 1] Shuriken
  (:`Pressed`
    (if (== (`self.CurrentUltCharge`) (`self.UltChargeRequired`))
      (`|SpawnActorFromClass` "/Game/Blueprints/Assassin/BP_Shuriken.BP_Shuriken_C" (`KismetMathLibrary.MakeTransform` _returnvalue_location _returnvalue_rotation (75.0 75.0 75.0)) "Undefined" "OverrideRootScale" null 0.0 0.0 5.0 self)
      (set `self.CurrentUltCharge` 0.0)
      (set `self.NormalizedUltCharge` 0.0))))

(fn `BoltProj`
  (bind (_returnvalue_location _returnvalue_rotation) (`KismetMathLibrary.BreakTransform` (`SceneComponent.K2_GetComponentToWorld` (`self.ProjSpawnLoc`))))
  (`|SpawnActorFromClass` "/Game/Blueprints/Wizard/BP_Bolt.BP_Bolt_C" (`KismetMathLibrary.MakeTransform` _returnvalue_location _returnvalue_rotation) "Undefined" "OverrideRootScale" null 0.0 self))

(fn `UserConstructionScript`
  (`parent.UserConstructionScript`))