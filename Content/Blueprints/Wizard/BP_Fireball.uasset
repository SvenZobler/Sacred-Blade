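; BP_Fireball is the Wizard's fireball, which damages the boss and leaves a fire patch on impact.
; Sphere overlap with BP_Boss triggers a damage flash, adds ult charge to the instigating player and deals damage.
; Boss, Wall or Floor hits trace downward to place BP_FirePatch with its patch damage, then destroy the fireball.
; Boss hits offset the patch toward the boss and pass the player reference.
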(event `self.ReceiveBeginPlay`
  (`SceneComponent.SetWorldScale3D` (`self.Sphere1`) (1.0 1.0 1.0)))

(event `self.Sphere1.OnComponentBeginOverlap`
  (params (OverlappedComponent :type "PrimitiveComponent Object Reference") (OtherActor :type "Actor Object Reference") (OtherComp :type "PrimitiveComponent Object Reference") (OtherBodyIndex :type Integer) (bFromSweep :type Boolean) (SweepResult :type "HitResult Structure (by ref)"))
  (bind _returnvalue (`self.K2_GetActorLocation`))
  (`/Engine/EditorBlueprintResources/StandardMacros.IsValid` OtherActor
    (:`Is Valid`
      (bind _asbp_boss (cast `/Game/Blueprints/BP_Boss` OtherActor)
        (:`then`
          ;[1 1 1] Damage Feedback
          (`/Game/Blueprints/BP_Boss.DamageFlash` _asbp_boss)
          ;[1 1 1] Add Ult Charge
          (bind _asbp_player_parent (cast `/Game/Blueprints/BP_Player_Parent` (`self.Instigator`))
            (:`then`
              (`/Game/Blueprints/BP_Player_Parent.AddUltCharge` _asbp_player_parent (`self.FireballDamage`)))
            (:`CastFailed`
              _))
          ;[1 1 1] TakeDamage
          (`/Game/Blueprints/BP_Boss.TakeDamage` _asbp_boss (`self.FireballDamage`))
          (bind _outhit (`KismetSystemLibrary.LineTraceSingleForObjects` _returnvalue (- _returnvalue (0.0 0.0 1000.0)) (`|MakeArray` "ObjectTypeQuery8" :!type "EObjectTypeQuery Enum")))
          (`|SpawnActorFromClass` "/Game/Blueprints/Wizard/BP_FirePatch.BP_FirePatch_C" (`KismetMathLibrary.MakeTransform` (+ (`.Location` (`GameplayStatics.BreakHitResult` _outhit)) (* (`KismetMathLibrary.GetDirectionUnitVector` (`self.K2_GetActorLocation`) (`self.K2_GetActorLocation` _asbp_boss)) 150.0))) "Undefined" "OverrideRootScale" null (`self.FireballPatchDamage`) _asbp_player_parent (`self.Instigator`))
          (`self.K2_DestroyActor`))
        (:`CastFailed`
          (if (or (`self.ActorHasTag` OtherActor "Wall") (`self.ActorHasTag` OtherActor "Floor"))
            (bind _outhit_2 (`KismetSystemLibrary.LineTraceSingleForObjects` _returnvalue (- _returnvalue (0.0 0.0 1000.0)) (`|MakeArray` "ObjectTypeQuery8" :!type "EObjectTypeQuery Enum")))
            (`|SpawnActorFromClass` "/Game/Blueprints/Wizard/BP_FirePatch.BP_FirePatch_C" (`KismetMathLibrary.MakeTransform` (`.Location` (`GameplayStatics.BreakHitResult` _outhit_2))) "Undefined" "OverrideRootScale" null (`self.FireballPatchDamage`) null (`self.Instigator`))
            (`self.K2_DestroyActor`)))))))

(fn `UserConstructionScript`)